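; VR flashlight actor that the player can pick up, drop and switch on or off.
; Pickup disables physics, snaps it to the motion controller at a grip offset, sets the hand pose, and clears the other hand's hold when swapping hands.
; Drop detaches it, re-enables physics and updates the hand animation.
; Interact uses a FlipFlop to toggle the spotlight and the mesh material's light intensity together.
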(event EventBeginPlay)

(event Collision|EventActorBeginOverlap
  (params (OtherActor :type Actor%20Object%20Reference)))

(event EventTick
  (params (DeltaSeconds :type Float%20%28single-precision%29)))

(event EventPickup
  (params (AttachTo :type Scene%20Component%20Object%20Reference))
  (bind _self self)
  (bind _staticmeshcomponent (Variables|Debug|GetStaticMeshComponent))
  (Physics|SetSimulatePhysics _staticmeshcomponent false)
  (Transformation|AttachComponentToComponent (VehicleSound|GetRootComponent) AttachTo "None" "SnapToTarget" "SnapToTarget" "KeepWorld" false)
  (Transformation|SetRelativeLocationAndRotation _staticmeshcomponent "0.491153,0.000000,-0.073287" "-0.000000,90.000000,-145.000000" false false)
  (Default|SetHandAnim (Variables|Default|GetActorComponent_SetHandAnimation) (Variables|Default|GetAnimationToUse) AttachTo (Variables|Default|GetBlend%20Space%20to%20Use) true)
  (bind _asvrplayer_no_ui (Utilities|Casting|CastToVRPlayerNoUI (Game|GetPlayerCharacter 0)))
  (if (== AttachTo (Variables|/Game/VirtualRealityBP/Blueprints/BP_MotionControllerNoUI.BP_MotionControllerNoUI_C|GetMotionController (Variables|/Game/VirtualRealityBP/Blueprints/VRPlayerNoUI.VRPlayerNoUI_C|GetLeftController _asvrplayer_no_ui)))
    (if (== _self (Variables|/Game/VirtualRealityBP/Blueprints/BP_MotionControllerNoUI.BP_MotionControllerNoUI_C|GetAttachedActor (Variables|/Game/VirtualRealityBP/Blueprints/VRPlayerNoUI.VRPlayerNoUI_C|GetRightController _asvrplayer_no_ui)))
      (Variables|/Game/VirtualRealityBP/Blueprints/BP_MotionControllerNoUI.BP_MotionControllerNoUI_C|SetAttachedActor (Variables|/Game/VirtualRealityBP/Blueprints/VRPlayerNoUI.VRPlayerNoUI_C|GetRightController _asvrplayer_no_ui) 0)
      (bind _asarmblend_bp (Utilities|Casting|CastToarmblend_BP (Components|SkeletalMesh|GetAnimInstance (Variables|/Game/VirtualRealityBP/Blueprints/BP_MotionControllerNoUI.BP_MotionControllerNoUI_C|GetHandMesh (Variables|/Game/VirtualRealityBP/Blueprints/VRPlayerNoUI.VRPlayerNoUI_C|GetRightController _asvrplayer_no_ui)))))
      (Variables|/Game/Hands/Animation/armblend_BP.armblend_BP_C|SetSwitch%20Animation _asarmblend_bp true))
    (elif (== _self (Variables|/Game/VirtualRealityBP/Blueprints/BP_MotionControllerNoUI.BP_MotionControllerNoUI_C|GetAttachedActor (Variables|/Game/VirtualRealityBP/Blueprints/VRPlayerNoUI.VRPlayerNoUI_C|GetLeftController _asvrplayer_no_ui)))
      (Variables|/Game/VirtualRealityBP/Blueprints/BP_MotionControllerNoUI.BP_MotionControllerNoUI_C|SetAttachedActor (Variables|/Game/VirtualRealityBP/Blueprints/VRPlayerNoUI.VRPlayerNoUI_C|GetLeftController _asvrplayer_no_ui) 0)
      (bind _asarmblend_bp_2 (Utilities|Casting|CastToarmblend_BP (Components|SkeletalMesh|GetAnimInstance (Variables|/Game/VirtualRealityBP/Blueprints/BP_MotionControllerNoUI.BP_MotionControllerNoUI_C|GetHandMesh (Variables|/Game/VirtualRealityBP/Blueprints/VRPlayerNoUI.VRPlayerNoUI_C|GetLeftController _asvrplayer_no_ui)))))
      (Variables|/Game/Hands/Animation/armblend_BP.armblend_BP_C|SetSwitch%20Animation _asarmblend_bp_2 true))))

(event EventDrop
  (Physics|SetSimulatePhysics (Variables|Debug|GetStaticMeshComponent) true)
  (Transformation|DetachFromActor "KeepWorld" "KeepWorld" "KeepWorld")
  (Default|SetHandAnim (Variables|Default|GetActorComponent_SetHandAnimation) "NewEnumerator0" (stale EventPickup AttachTo) (Variables|Default|GetBlend%20Space%20to%20Use) false))

(event EventInteract
  (bind _staticmeshcomponent (Variables|Debug|GetStaticMeshComponent))
  (bind _spotlight (Variables|Default|GetSpotLight))
  (bind _isa (Utilities|FlowControl|FlipFlop)
    (:A
      (Variables|Default|SetFlashlightOn _isa)
      (Rendering|Components|Light|SetIntensity _spotlight 5e+03)
      (Rendering|Material|SetScalarParameterValueonMaterials _staticmeshcomponent "LightIntensity" 1e+01))
    (:B
      (Variables|Default|SetFlashlightOn _isa)
      (Rendering|Components|Light|SetIntensity _spotlight 0.0)
      (Rendering|Material|SetScalarParameterValueonMaterials _staticmeshcomponent "LightIntensity" 0.0))))

(fn ConstructionScript)
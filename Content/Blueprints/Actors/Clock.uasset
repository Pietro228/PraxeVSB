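; Clock actor that displays the current system time by rotating two hand components.
; On every Tick it reads Now and sets the relative pitch of both hands.
; Rucicka is the minute hand, sweeping a full turn per hour from the combined minutes and seconds.
; Rucicka1 is the hour hand, stepping thirty degrees per hour plus the elapsed fraction of the current hour.
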(event EventBeginPlay)

(event Collision|EventActorBeginOverlap
  (params (OtherActor :type Actor%20Object%20Reference)))

(event EventTick
  (params (DeltaSeconds :type Float%20%28single-precision%29))
  (bind _returnvalue (Math|DateTime|Now))
  (bind _returnvalue_2 (Math|DateTime|Now))
  (Transformation|SetRelativeRotation (Variables|Default|GetRucicka) (Math|Rotator|MakeRotator 0.0 (* (Math|Float|NormalizetoRange (Math|Conversions|ToFloat(Integer) (+ (Class|KismetMathLibrary|GetSecond _returnvalue_2) (* (Class|KismetMathLibrary|GetMinute _returnvalue_2) 60))) 0.0 3.6e+03) -3.6e+02) 0.0) false false)
  (Transformation|SetRelativeRotation (Variables|Default|GetRucicka1) (Math|Rotator|MakeRotator 0.0 (+ (* (Math|Float|NormalizetoRange (Math|Conversions|ToFloat(Integer) (+ (Class|KismetMathLibrary|GetSecond _returnvalue) (* (Class|KismetMathLibrary|GetMinute _returnvalue) 60))) 0.0 3.6e+03) -3e+01) (* (Class|KismetMathLibrary|GetHour _returnvalue) -30)) 0.0) false false))

(fn ConstructionScript)
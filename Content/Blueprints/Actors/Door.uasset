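; Double door actor that swings open or closed when its linked KeypadLock reports a successful code submission.
; Every Tick, if the keypad is valid, it binds OpenCloseDoor to the keypad's submit-success event.
; OpenCloseDoor toggles the Opening flag and plays or reverses the OpenClose timeline, which yaws the DvereL and DvereP leaves in mirrored directions.
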(event Custom|OpenCloseDoor
  (if (Variables|Default|GetOpening)
    (Variables|Default|SetOpening false)
    (bind _value (Timeline|OpenClose Reverse)
      (:Update
        (Transformation|SetRelativeRotation (Variables|Default|GetdvereL) (Math|Rotator|MakeRotator 0.0 0.0 (Math|Float|Lerp 0.0 95.0 _value)) false false)
        (Transformation|SetRelativeRotation (Variables|Default|GetdvereP) (Math|Rotator|MakeRotator 0.0 0.0 (* (Math|Float|Lerp 0.0 95.0 _value) -1.0)) false false)))
    (else
      (Variables|Default|SetOpening true)
      (Timeline|OpenClose Play))))

(event EventTick
  (params (DeltaSeconds :type Float%20%28single-precision%29))
  (bind _keypadlock (Variables|Settings|GetKeypadLock))
  (Utilities|IsValid _keypadlock
    (:Is%20Valid
      (EventDispatchers|BindEventtoOnSubmitSuccess _keypadlock (delegate Custom|OpenCloseDoor)))))

(fn ConstructionScript)
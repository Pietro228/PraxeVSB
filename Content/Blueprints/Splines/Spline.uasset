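; Spline actor that builds a chain of deformed spline mesh segments along its spline in the construction script.
; It divides the spline length by SectionLength and adds one collision-enabled spline mesh per whole section, leaving any remainder uncovered.
; Each segment takes its endpoints and tangents from the spline, with tangents clamped to the section length, then gets a random relative roll on the whole component.
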(event EventBeginPlay)

(event Collision|EventActorBeginOverlap
  (params (OtherActor :type Actor%20Object%20Reference)))

(event EventTick
  (params (DeltaSeconds :type Float%20%28single-precision%29)))

(fn ConstructionScript
  (bind _spline (Variables|Default|GetSpline))
  (bind _sectionlength (LocalVariables|GetSectionLength))
  (for _index (range 0 (- (Math|Float|Truncate (/ (Spline|GetSplineLength (Variables|Default|GetSpline)) (LocalVariables|GetSectionLength))) 1))
    (bind _returnvalue (AddComponent|AddSplineMeshComponent false))
    (SplineMesh|SetForwardAxis _returnvalue "X" true)
    (SplineMesh|SetStartandEnd _returnvalue (Spline|GetLocationatDistanceAlongSpline _spline (* _index _sectionlength) "Local") (Math|Vector|ClampVectorSize (Spline|GetTangentatDistanceAlongSpline _spline (* _index _sectionlength) "Local") 0.0 (LocalVariables|GetSectionLength)) (Spline|GetLocationatDistanceAlongSpline _spline (* (+ _index 1) _sectionlength) "Local") (Math|Vector|ClampVectorSize (Spline|GetTangentatDistanceAlongSpline _spline (* (+ _index 1) _sectionlength) "Local") 0.0 (LocalVariables|GetSectionLength)) true :!class /Script/Engine.SplineMeshComponent)
    (Collision|SetCollisionEnabled _returnvalue "QueryAndPhysics")
    (Transformation|SetRelativeRotation _returnvalue (Math|Rotator|MakeRotator (Math|Random|RandomFloatinRange 0.0 3.6e+02) 0.0 0.0) false false)))